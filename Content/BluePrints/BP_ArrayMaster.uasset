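; BP_ArrayMaster filters data table records by the sex, age group and topic picked in three UI widgets and sends matching indices to BP_PointMaker.
; On BeginPlay it caches those references and sorts 50 DataTableTest rows into per-category index sets.
; IntersectionEvent intersects the selected sets, treating -1 as all rows, then calls SetWaitPoint with the result.
; When all three selections are -1, it sends NullSet instead.
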(event Custom|IntersectionEvent
  (CallFunction|MakeSelectArray)
  (CallFunction|IntersectionArray (Variables|Default|GetselectIntArray)))

(event EventBeginPlay
  (CallFunction|GetValue)
  (for _index (range 1 50)
    (bind _returnvalue (Utilities|GetDataTableRow "/Game/Data_Temp/DataTableTest.DataTableTest" (Utilities|String|StringToName (Utilities|String|ToString(Integer) _index)))
      (:then
        (Utilities|FlowControl|Sequence
          (:then_0
            (CallFunction|SexMakeArray (- _index 1) (.sex (Utilities|Struct|BreakmovieStruct _returnvalue))))
          (:then_1
            (CallFunction|AgeMakeArray (- _index 1) (- (/ (.age (Utilities|Struct|BreakmovieStruct _returnvalue)) 10) 1)))
          (:then_2
            (CallFunction|TopicMakeArray (- _index 1) (.topic (Utilities|Struct|BreakmovieStruct _returnvalue))))
          (:then_3
            (Utilities|Set|Add (Variables|Default|GetAllnullset) (- _index 1))))))))

(fn ConstructionScript)

(fn SexMakeArray
  (params (index :type Integer) (sexInt :type Integer))
  (if (== sexInt 0)
    (Utilities|Set|Add (Variables|Default|Getsex_Man_Set) index)
    (else
      (Utilities|Set|Add (Variables|Default|Getsex_Woman_Set) index))))

(fn AgeMakeArray
  (params (index :type Integer) (ageInt :type Integer))
  (switch Utilities|FlowControl|Switch|SwitchonAgeEnum (Utilities|Enum|ByteToEnumAgeEnum (Math|Conversions|ToByte(Integer) ageInt))
    (:NewEnumerator0
      (Utilities|Set|Add (Variables|Default|Getage_10_Set) index))
    (:NewEnumerator1
      (Utilities|Set|Add (Variables|Default|Getage_20_Set) index))
    (:NewEnumerator2
      (Utilities|Set|Add (Variables|Default|Getage_30_Set) index))
    (:NewEnumerator3
      (Utilities|Set|Add (Variables|Default|Getage_40_Set) index))
    (:NewEnumerator4
      (Utilities|Set|Add (Variables|Default|Getage_50_Set) index))))

(fn TopicMakeArray
  (params (index :type Integer) (topicInt :type Integer))
  (switch Utilities|FlowControl|Switch|SwitchonTopicEnum (Utilities|Enum|ByteToEnumTopicEnum (Math|Conversions|ToByte(Integer) topicInt))
    (:NewEnumerator0
      (Utilities|Set|Add (Variables|Default|Gettopic_00_Set) index))
    (:NewEnumerator1
      (Utilities|Set|Add (Variables|Default|Gettopic_01_Set) index))
    (:NewEnumerator2
      (Utilities|Set|Add (Variables|Default|Gettopic_02_Set) index))
    (:NewEnumerator3
      (Utilities|Set|Add (Variables|Default|Gettopic_03_Set) index))
    (:NewEnumerator4
      (Utilities|Set|Add (Variables|Default|Gettopic_04_Set) index))
    (:NewEnumerator5
      (Utilities|Set|Add (Variables|Default|Gettopic_05_Set) index))
    (:NewEnumerator6
      (Utilities|Set|Add (Variables|Default|Gettopic_06_Set) index))
    (:NewEnumerator7
      (Utilities|Set|Add (Variables|Default|Gettopic_07_Set) index))
    (:NewEnumerator8
      (Utilities|Set|Add (Variables|Default|Gettopic_08_Set) index))
    (:NewEnumerator9
      (Utilities|Set|Add (Variables|Default|Gettopic_09_Set) index))))

(fn UnionArray
  (params (setButtonInt :type Array%20of%20Integers)))

(fn IntersectionArray
  (params (setButtonInt :type Array%20of%20Integers))
  (Utilities|FlowControl|Sequence
    (:then_0
      (CallFunction|SexSelectArray (Utilities|Array|Get(acopy) setButtonInt)))
    (:then_1
      (CallFunction|AgeSelectArray (Utilities|Array|Get(acopy) setButtonInt 1)))
    (:then_2
      (CallFunction|TopicSelectArray (Utilities|Array|Get(acopy) setButtonInt 2)))
    (:then_3
      (if (== (+ (Utilities|Array|Get(acopy) setButtonInt) (Utilities|Array|Get(acopy) setButtonInt 1) (Utilities|Array|Get(acopy) setButtonInt 2)) -3)
        (bind _output_get (Variables|Default|SetresultSet (Variables|Default|GetnullSet)))
        (bind _result (Utilities|Set|ToArray _output_get))
        (Default|SetWaitPoint (Variables|Default|Getbp_pm) _result)
        (else
          (bind _result_2 (Utilities|Set|Intersection (Variables|Default|GetsexSet) (Variables|Default|GetageSet)))
          (bind _result_3 (Utilities|Set|Intersection _result_2 (Variables|Default|GettopicSet)))
          (bind _output_get_2 (Variables|Default|SetresultSet _result_3))
          (bind _result_4 (Utilities|Set|ToArray _output_get_2))
          (Default|SetWaitPoint (Variables|Default|Getbp_pm) _result_4))))))

(fn SexSelectArray
  (params (selectInt :type Integer))
  (if (== selectInt -1)
    (Variables|Default|SetsexSet (Variables|Default|GetAllnullset))
    (elif (== selectInt 0)
      (Variables|Default|SetsexSet (Variables|Default|Getsex_Man_Set))
      (else
        (Variables|Default|SetsexSet (Variables|Default|Getsex_Woman_Set))))))

(fn AgeSelectArray
  (params (selectInt :type Integer))
  (if (== selectInt -1)
    (Variables|Default|SetageSet (Variables|Default|GetAllnullset))
    (else
      (switch Utilities|FlowControl|Switch|SwitchonAgeEnum (Utilities|Enum|ByteToEnumAgeEnum (Math|Conversions|ToByte(Integer) selectInt))
        (:NewEnumerator0
          (Variables|Default|SetageSet (Variables|Default|Getage_10_Set)))
        (:NewEnumerator1
          (Variables|Default|SetageSet (Variables|Default|Getage_20_Set)))
        (:NewEnumerator2
          (Variables|Default|SetageSet (Variables|Default|Getage_30_Set)))
        (:NewEnumerator3
          (Variables|Default|SetageSet (Variables|Default|Getage_40_Set)))
        (:NewEnumerator4
          (Variables|Default|SetageSet (Variables|Default|Getage_50_Set)))))))

(fn TopicSelectArray
  (params (selectInt :type Integer))
  (if (== selectInt -1)
    (Variables|Default|SettopicSet (Variables|Default|GetAllnullset))
    (else
      (switch Utilities|FlowControl|Switch|SwitchonTopicEnum (Utilities|Enum|ByteToEnumTopicEnum (Math|Conversions|ToByte(Integer) selectInt))
        (:NewEnumerator0
          (Variables|Default|SettopicSet (Variables|Default|Gettopic_00_Set)))
        (:NewEnumerator1
          (Variables|Default|SettopicSet (Variables|Default|Gettopic_01_Set)))
        (:NewEnumerator2
          (Variables|Default|SettopicSet (Variables|Default|Gettopic_02_Set)))
        (:NewEnumerator3
          (Variables|Default|SettopicSet (Variables|Default|Gettopic_03_Set)))
        (:NewEnumerator4
          (Variables|Default|SettopicSet (Variables|Default|Gettopic_04_Set)))
        (:NewEnumerator5
          (Variables|Default|SettopicSet (Variables|Default|Gettopic_05_Set)))
        (:NewEnumerator6
          (Variables|Default|SettopicSet (Variables|Default|Gettopic_06_Set)))
        (:NewEnumerator7
          (Variables|Default|SettopicSet (Variables|Default|Gettopic_07_Set)))
        (:NewEnumerator8
          (Variables|Default|SettopicSet (Variables|Default|Gettopic_08_Set)))
        (:NewEnumerator9
          (Variables|Default|SettopicSet (Variables|Default|Gettopic_09_Set)))))))

(fn MakeSelectArray
  (bind _selectintarray (Variables|Default|GetselectIntArray))
  (Utilities|Array|Clear (Variables|Default|GetselectIntArray))
  (Utilities|Array|Add _selectintarray (Variables|/Game/VRUI/WBP_SexUI.WBP_SexUI_C|GetselectSexIndex (Variables|Default|GetwbpSexUI)))
  (Utilities|Array|Add _selectintarray (Variables|/Game/VRUI/WBP_AgeUI.WBP_AgeUI_C|GetselectAgeIndex (Variables|Default|GetwbpAgeUI)))
  (Utilities|Array|Add _selectintarray (Variables|/Game/VRUI/WBP_TopicUI.WBP_TopicUI_C|GetselectTopicIndex (Variables|Default|GetwbpTopicUI))))

(fn GetValue
  (bind _outactors (Actor|GetAllActorsOfClass "/Game/BluePrints/BP_PointMaker.BP_PointMaker_C"))
  (Variables|Default|Setbp_pm (Utilities|Array|Get(acopy) _outactors))
  (Utilities|FlowControl|Sequence
    (:then_0
      (bind _outactors_2 (Actor|GetAllActorsOfClass "/Game/VRUI/BP_SexUI.BP_SexUI_C"))
      (bind _aswbp_sex_ui (Utilities|Casting|CastToWBP_SexUI (UserInterface|GetWidget (Variables|/Game/VRUI/BP_SexUI.BP_SexUI_C|GetWidget (Utilities|Array|Get(acopy) _outactors_2)))))
      (Variables|Default|SetwbpSexUI _aswbp_sex_ui))
    (:then_1
      (bind _outactors_3 (Actor|GetAllActorsOfClass "/Game/VRUI/BP_AgeUI.BP_AgeUI_C"))
      (bind _aswbp_age_ui (Utilities|Casting|CastToWBP_AgeUI (UserInterface|GetWidget (Variables|/Game/VRUI/BP_AgeUI.BP_AgeUI_C|GetWidget (Utilities|Array|Get(acopy) _outactors_3)))))
      (Variables|Default|SetwbpAgeUI _aswbp_age_ui))
    (:then_2
      (bind _outactors_4 (Actor|GetAllActorsOfClass "/Game/VRUI/BP_Topic.BP_Topic_C"))
      (bind _aswbp_topic_ui (Utilities|Casting|CastToWBP_TopicUI (UserInterface|GetWidget (Variables|/Game/VRUI/BP_Topic.BP_Topic_C|GetWidget (Utilities|Array|Get(acopy) _outactors_4)))))
      (Variables|Default|SetwbpTopicUI _aswbp_topic_ui))))