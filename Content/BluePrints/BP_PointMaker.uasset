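; Spawner and coordinator for a VR flock of textured planes, some filled from data table rows, the rest dummies.
; Planes spawn in a wall grid, each targeting a point actor that Tick moves along BP_BoidsTemp's particle positions and velocities.
; SetWaitPoint sends selected data planes to wait points on a curved grid around the player, facing them, and returns the others to the flock.
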(event Custom|SetWaitPoint
  (params (indexArray :type Array%20of%20Integers))
  ;[1 1 1] PosSetting
  (for (_array_element _array_index) (Variables|Default|GetplaneActorArray)
    (Variables|Default|SetselectPlane _array_element)
    (if (== (Utilities|Array|FindItem indexArray _array_index) -1)
      ;;[1 1 1] Boid로 돌아가라
      (Default|GoBoids (Variables|Default|GetselectPlane))
      (Variables|/Game/BluePrints/BP_Plane.BP_Plane_C|SettargetActor (Variables|Default|GetselectPlane) (Utilities|Array|Get(acopy) (Variables|Default|GetboidsPointArray) _array_index))
      (else
        (CallFunction|MakeWaitPosCal indexArray)
        (Default|GoWait (Variables|Default|GetselectPlane))
        (Variables|/Game/BluePrints/BP_Plane.BP_Plane_C|SettargetActor (Variables|Default|GetselectPlane) (Utilities|Array|Get(acopy) (Variables|Default|GetwaitPointArray) _array_index))))))

(event EventBeginPlay
  (CallFunction|StartPosSettingF)
  (CallFunction|StartSetting))

(event EventTick
  (params (DeltaSeconds :type Float%20%28single-precision%29))
  (CallFunction|SetBoidsPos))

(fn ConstructionScript)

(fn StartSetting
  (bind _texturearray (Variables|Default|GettextureArray))
  (bind _outactors (Actor|GetAllActorsOfClass "/Game/Boids/BP_BoidsTemp.BP_BoidsTemp_C"))
  (Variables|Default|SetmyBoids (Utilities|Array|Get(acopy) _outactors))
  (Variables|Default|SetmyVRPlayer (Game|Player|GetPlayerPawn 0))
  (for _index (range 0 49)
    (bind _returnvalue (Game|SpawnActorfromClass "/Game/BluePrints/BP_BoidsPoint.BP_BoidsPoint_C" (Math|Transform|MakeTransform "0, 0, 0" "0, 0, 0" "1,1,1") "Undefined" 0 0))
    (Utilities|Array|Add (Variables|Default|GetboidsPointArray) _returnvalue)
    (bind _returnvalue_2 (Game|SpawnActorfromClass "/Game/BluePrints/BP_WaitPoint.BP_WaitPoint_C" (Math|Transform|MakeTransform "0, 0, 0" "0, 0, 0" "1,1,1") "Undefined" 0 0))
    (Utilities|Array|Add (Variables|Default|GetwaitPointArray) _returnvalue_2)
    (CallFunction|SettingPlane (+ _index 1)))
  ;[1 1 1] Make Dummy
  (for _index_2 (range 0 449)
    (bind _returnvalue_3 (Game|SpawnActorfromClass "/Game/BluePrints/BP_BoidsPoint.BP_BoidsPoint_C" (Math|Transform|MakeTransform "0, 0, 0" "0, 0, 0" "1,1,1") "Undefined" 0 0))
    (Utilities|Array|Add (Variables|Default|GetboidsPointArray) _returnvalue_3)
    (bind _returnpos (CallFunction|SetPos (+ _index_2 50)))
    (bind _returnvalue_4 (Game|SpawnActorfromClass "/Game/BluePrints/BP_Plane_Child.BP_Plane_Child_C" (Math|Transform|MakeTransform _returnpos "0, 0, 0" "1,1,1") "Undefined" 0 0))
    (Variables|/Game/BluePrints/BP_Plane.BP_Plane_C|SettargetActor _returnvalue_4 _returnvalue_3)
    (Default|GoStartWait _returnvalue_4 (Math|Random|RandomFloatinRange 11.0 13.0) (Math|Random|RandomFloatinRange 3.0 5.0))
    (Default|SetTexture _returnvalue_4 (Utilities|Array|Get(acopy) _texturearray (Math|Integer|%(Integer) _index_2 (Utilities|Array|Length _texturearray))))))

(fn SettingPlane
  (params (index :type Integer))
  (bind _returnvalue (- index 1))
  (bind _texturearray (Variables|Default|GettextureArray))
  (bind _returnvalue_2 (Utilities|GetDataTableRow "/Game/Data_Temp/DataTableTest.DataTableTest" (Utilities|String|StringToName (Utilities|String|ToString(Integer) index)))
    (:then
      (Utilities|FlowControl|Sequence
        (:then_0
          (bind _returnpos (CallFunction|SetPos (- index 1)))
          (bind _returnvalue_3 (Game|SpawnActorfromClass "/Game/BluePrints/BP_Plane.BP_Plane_C" (Math|Transform|MakeTransform _returnpos "0, 0, 0" "1,1,1") "Undefined" 0 0))
          (Variables|/Game/BluePrints/BP_Plane.BP_Plane_C|SettargetActor _returnvalue_3 (Utilities|Array|Get(acopy) (Variables|Default|GetboidsPointArray) _returnvalue))
          (Default|GoStartWait _returnvalue_3 (Math|Random|RandomFloatinRange 11.0 13.0) (Math|Random|RandomFloatinRange 3.0 5.0))
          (Utilities|Array|Add (Variables|Default|GetplaneActorArray) _returnvalue_3)
          (Default|SetTexture _returnvalue_3 (Utilities|Array|Get(acopy) _texturearray (Math|Integer|%(Integer) _returnvalue (Utilities|Array|Length _texturearray)))))
        (:then_1
          (Default|SetColor _returnvalue_3 (.sex (Utilities|Struct|BreakmovieStruct _returnvalue_2))))
        (:then_2
          (Default|SetAge _returnvalue_3 (.age (Utilities|Struct|BreakmovieStruct _returnvalue_2))))
        (:then_3
          (Default|SetTopic _returnvalue_3 (+ (.topic (Utilities|Struct|BreakmovieStruct _returnvalue_2)) 1)))))))

(fn MakeWaitPosCal
  (params (selectIndexArray :type Array%20of%20Integers))
  (bind _returnvalue (Utilities|Array|Length selectIndexArray))
  (bind _horizontallenght (Variables|Default|GetHorizontalLenght))
  (bind _planeangle (Variables|Default|GetplaneAngle))
  (Variables|Default|SetwaitStart_Pos (+ (+ (Transformation|GetActorLocation) (* (Transformation|GetActorForwardVector) -3e+02)) "0, 0, 0"))
  (Variables|Default|SetmyMatrix (Utilities|Struct|MakeIntVector (Math|Integer|Clamp(Integer) _returnvalue 0 (Variables|Default|GetHorizontalLenght)) (Math|Conversions|ToInteger(Byte) (Class|KismetMathLibrary|FFloor64 (/ (Math|Conversions|ToFloat(Integer) _returnvalue) (+ (Math|Conversions|ToFloat(Integer) (Variables|Default|GetHorizontalLenght)) 0.001)))) 0))
  (for (_array_element _array_index) selectIndexArray
    (bind _asbp_wait_point (Utilities|Casting|CastToBP_WaitPoint (Utilities|Array|Get(acopy) (Variables|Default|GetwaitPointArray) _array_element)))
    (Variables|/Game/BluePrints/BP_WaitPoint.BP_WaitPoint_C|SetgoalPos _asbp_wait_point (+ (+ (Transformation|GetActorLocation (Variables|Default|GetmyVRPlayer)) (* (Math|Vector|VectorUp) 1.5e+02)) (* (Math|Vector|RotateVector "1.000000, 0, 0" (Math|Rotator|MakeRotator 0.0 (* (.pitch _planeangle) (- (* (Math|Conversions|ToFloat(Integer) (.y (Variables|Default|GetmyMatrix))) 0.5) (Math|Conversions|ToFloat(Integer) (/ _array_index _horizontallenght)))) (* (.yaw _planeangle) (+ (Math|Conversions|ToFloat(Integer) (Math|Integer|%(Integer) _array_index _horizontallenght)) (* (Math|Conversions|ToFloat(Integer) (- (.x (Variables|Default|GetmyMatrix)) 1)) -0.5))))) (Variables|Default|GetwaitPosLenght))))
    (Variables|/Game/BluePrints/BP_WaitPoint.BP_WaitPoint_C|SetstartPos _asbp_wait_point (+ (+ (Transformation|GetActorLocation (Variables|Default|GetmyVRPlayer)) (* (Math|Vector|VectorUp) 1.5e+02)) (* (Math|Vector|RotateVector "1.000000, 0, 0" (Math|Rotator|MakeRotator 0.0 (* (.pitch _planeangle) (- (* (Math|Conversions|ToFloat(Integer) (.y (Variables|Default|GetmyMatrix))) 0.5) (Math|Conversions|ToFloat(Integer) (/ _array_index _horizontallenght)))) (* (.yaw _planeangle) (+ (Math|Conversions|ToFloat(Integer) (Math|Integer|%(Integer) _array_index _horizontallenght)) (* (Math|Conversions|ToFloat(Integer) (- (.x (Variables|Default|GetmyMatrix)) 1)) -0.5))))) (Variables|Default|GetwaitPosLenght))))
    (Variables|/Game/BluePrints/BP_WaitPoint.BP_WaitPoint_C|SetoriginPos _asbp_wait_point (+ (+ (Transformation|GetActorLocation (Variables|Default|GetmyVRPlayer)) (* (Math|Vector|VectorUp) 1.5e+02)) (* (Math|Vector|RotateVector "1.000000, 0, 0" (Math|Rotator|MakeRotator 0.0 (* (.pitch _planeangle) (- (* (Math|Conversions|ToFloat(Integer) (.y (Variables|Default|GetmyMatrix))) 0.5) (Math|Conversions|ToFloat(Integer) (/ _array_index _horizontallenght)))) (* (.yaw _planeangle) (+ (Math|Conversions|ToFloat(Integer) (Math|Integer|%(Integer) _array_index _horizontallenght)) (* (Math|Conversions|ToFloat(Integer) (- (.x (Variables|Default|GetmyMatrix)) 1)) -0.5))))) (Variables|Default|GetwaitPosLenght))))
    (Transformation|SetActorLocation (Utilities|Array|Get(acopy) (Variables|Default|GetwaitPointArray) _array_element) (+ (+ (Transformation|GetActorLocation (Variables|Default|GetmyVRPlayer)) (* (Math|Vector|VectorUp) 1.5e+02)) (* (Math|Vector|RotateVector "1.000000, 0, 0" (Math|Rotator|MakeRotator 0.0 (* (.pitch _planeangle) (- (* (Math|Conversions|ToFloat(Integer) (.y (Variables|Default|GetmyMatrix))) 0.5) (Math|Conversions|ToFloat(Integer) (/ _array_index _horizontallenght)))) (* (.yaw _planeangle) (+ (Math|Conversions|ToFloat(Integer) (Math|Integer|%(Integer) _array_index _horizontallenght)) (* (Math|Conversions|ToFloat(Integer) (- (.x (Variables|Default|GetmyMatrix)) 1)) -0.5))))) (Variables|Default|GetwaitPosLenght))) false false)
    (Transformation|SetActorRotation (Utilities|Array|Get(acopy) (Variables|Default|GetwaitPointArray) _array_element) (Math|Rotator|FindLookatRotation (+ (+ (Transformation|GetActorLocation (Variables|Default|GetmyVRPlayer)) (* (Math|Vector|VectorUp) 1.5e+02)) (* (Math|Vector|RotateVector "1.000000, 0, 0" (Math|Rotator|MakeRotator 0.0 (* (.pitch _planeangle) (- (* (Math|Conversions|ToFloat(Integer) (.y (Variables|Default|GetmyMatrix))) 0.5) (Math|Conversions|ToFloat(Integer) (/ _array_index _horizontallenght)))) (* (.yaw _planeangle) (+ (Math|Conversions|ToFloat(Integer) (Math|Integer|%(Integer) _array_index _horizontallenght)) (* (Math|Conversions|ToFloat(Integer) (- (.x (Variables|Default|GetmyMatrix)) 1)) -0.5))))) (Variables|Default|GetwaitPosLenght))) (+ (Transformation|GetActorLocation (Variables|Default|GetmyVRPlayer)) (* (Math|Vector|VectorUp) 5e+01))))))

(fn MakeWaitPosRandom
  (params (index :type Integer))
  (Transformation|SetActorLocation (Utilities|Array|Get(acopy) (Variables|Default|GetwaitPointArray) index) (+ (Transformation|GetActorLocation) (* (Transformation|GetActorForwardVector) -3e+02) (Math|Vector|MakeVector (Math|Random|RandomFloatinRange -1e+01 1e+01) (Math|Random|RandomFloatinRange -2e+02 2e+02) (Math|Random|RandomFloatinRange -2e+02 2e+02))) false false))

(fn SetBoidsPos
  (bind _myboids (Variables|Default|GetmyBoids))
  (for (_array_element _array_index) (Variables|Default|GetboidsPointArray)
    (Transformation|SetActorLocationAndRotation _array_element (Utilities|Array|Get(acopy) (Variables|/Game/Boids/BP_BoidsTemp.BP_BoidsTemp_C|GetparticlesPosArray _myboids) _array_index) (Math|Conversions|RotationFromXVector (Utilities|Array|Get(acopy) (Variables|/Game/Boids/BP_BoidsTemp.BP_BoidsTemp_C|GetparticleVelArray _myboids) _array_index)))))

(fn TestMove
  (params (index :type Array%20of%20Integers)))

(fn SetPos
  (params (index :type Integer))
  (bind _planesize (Variables|Default|GetplaneSize))
  (return (+ (Variables|Default|GetstartWaitPos) (Math|Vector|MakeVector 0.0 (* (Math|Integer|%(Integer) index 25) (.y _planesize)) (* (* (/ index 25) -1) (.z _planesize))))))

(fn StartPosSettingF
  (bind _planesize (Variables|Default|GetplaneSize))
  (Variables|Default|SetstartWaitPos (+ (Math|Vector|MakeVector 8e+02 0.0 3e+02) (Math|Vector|MakeVector (.x _planesize) (* (.y _planesize) -12.5) (* (.z _planesize) 1e+01)))))