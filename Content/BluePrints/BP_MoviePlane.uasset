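; BP_MoviePlane is an actor that shows video on a plane mesh, hidden when play begins.
; PlayVideo stores the given index, opens an entry from a media source list wrapped to four slots by modulo, and reveals the plane.
; StopVideo hides the plane and pauses the media player.
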(event Custom|PlayVideo
  (params (index :type Integer))
  (bind _output_get (Variables|Default|SetplayIndex index))
  (Media|MediaPlayer|OpenSource (Variables|Default|GetmediaPlayer) (Utilities|Array|Get(acopy) (Variables|Default|Getm_SourceList) (Math|Integer|%(Integer) _output_get 4)))
  (Rendering|SetVisibility (Variables|Default|GetPlane) true false))

(event Custom|StopVideo
  (Rendering|SetVisibility (Variables|Default|GetPlane) false false)
  (Sequencer|Player|Pause (Variables|Default|GetmediaPlayer)))

(event EventBeginPlay
  (Rendering|SetVisibility (Variables|Default|GetPlane) false false))

(event Collision|EventActorBeginOverlap
  (params (OtherActor :type Actor%20Object%20Reference)))

(event EventTick
  (params (DeltaSeconds :type Float%20%28single-precision%29)))

(fn ConstructionScript)