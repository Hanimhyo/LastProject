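; BP_StartSetting is a spawner actor that scatters roughly two thousand textured BP_Plane actors over a sphere around itself on BeginPlay.
; Each position comes from a normalized random vector at a fixed radius from the actor.
; Textures cycle through MyTextureList, with each plane scaled to its texture's aspect ratio, longest side normalized to one.
; A dynamic material instance per plane receives the image through the MainTexture parameter.
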(event EventBeginPlay
  (for _index (range 0 2000)
    (bind _returnvalue (Game|SpawnActorfromClass "/Game/BluePrints/BP_Plane.BP_Plane_C" (Math|Transform|MakeTransform (+ (Transformation|GetActorLocation) (* (Math|Vector|Normalize (Math|Vector|MakeVector (Math|Random|RandomFloatinRange -1.0 1.0) (Math|Random|RandomFloatinRange -1.0 1.0) (Math|Random|RandomFloatinRange -1.0 1.0))) 5e+02)) "0, 0, 0" (Math|Vector|MakeVector (/ (Math|Conversions|ToFloat(Integer) (Class|Texture2D|BlueprintGetSizeX (Utilities|Array|Get(acopy) (Variables|Default|GetmyTexture_List) (Math|Integer|%(Integer) _index (Utilities|Array|Length (Variables|Default|GetmyTexture_List)))))) (Math|Conversions|ToFloat(Integer) (Math|Integer|Max(Integer) (Class|Texture2D|BlueprintGetSizeX (Utilities|Array|Get(acopy) (Variables|Default|GetmyTexture_List) (Math|Integer|%(Integer) _index (Utilities|Array|Length (Variables|Default|GetmyTexture_List))))) (Class|Texture2D|BlueprintGetSizeY (Utilities|Array|Get(acopy) (Variables|Default|GetmyTexture_List) (Math|Integer|%(Integer) _index (Utilities|Array|Length (Variables|Default|GetmyTexture_List)))))))) (/ (Math|Conversions|ToFloat(Integer) (Class|Texture2D|BlueprintGetSizeY (Utilities|Array|Get(acopy) (Variables|Default|GetmyTexture_List) (Math|Integer|%(Integer) _index (Utilities|Array|Length (Variables|Default|GetmyTexture_List)))))) (Math|Conversions|ToFloat(Integer) (Math|Integer|Max(Integer) (Class|Texture2D|BlueprintGetSizeX (Utilities|Array|Get(acopy) (Variables|Default|GetmyTexture_List) (Math|Integer|%(Integer) _index (Utilities|Array|Length (Variables|Default|GetmyTexture_List))))) (Class|Texture2D|BlueprintGetSizeY (Utilities|Array|Get(acopy) (Variables|Default|GetmyTexture_List) (Math|Integer|%(Integer) _index (Utilities|Array|Length (Variables|Default|GetmyTexture_List)))))))) 1.0)) "Undefined" 0 0))
    (bind _returnvalue_2 (Rendering|Material|CreateDynamicMaterialInstance (Variables|/Game/BluePrints/BP_Plane.BP_Plane_C|GetPlane _returnvalue) 0 0 "None" :!class /Script/Engine.PrimitiveComponent))
    (Rendering|Material|SetTextureParameterValue _returnvalue_2 "MainTexture" (Utilities|Array|Get(acopy) (Variables|Default|GetmyTexture_List) (Math|Integer|%(Integer) _index (Utilities|Array|Length (Variables|Default|GetmyTexture_List)))))))

(event Collision|EventActorBeginOverlap
  (params (OtherActor :type Actor%20Object%20Reference)))

(event EventTick
  (params (DeltaSeconds :type Float%20%28single-precision%29)))

(fn ConstructionScript)