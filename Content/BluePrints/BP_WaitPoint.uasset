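; BP_WaitPoint is an actor that drifts continuously between random points close to a stored origin position.
; Tick advances an alpha over roughly two seconds and linearly interpolates the actor's location from start to goal, without sweeping.
; When the alpha passes one, it resets, takes the current location as the new start and picks a goal a short, fixed distance from the origin.
; Nothing in these graphs initializes the origin.
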(event EventBeginPlay)

(event Collision|EventActorBeginOverlap
  (params (OtherActor :type Actor%20Object%20Reference)))

(event EventTick
  (params (DeltaSeconds :type Float%20%28single-precision%29))
  (bind _output_get (Variables|Default|SetcurrentAlpha (+ (* DeltaSeconds 0.5) (Variables|Default|GetcurrentAlpha))))
  (if (> _output_get 1.0)
    (Variables|Default|SetcurrentAlpha 0.0)
    (Variables|Default|SetgoalPos (+ (Variables|Default|GetoriginPos) (* (Math|Random|RandomUnitVector) 1e+01)))
    (Variables|Default|SetstartPos (Transformation|GetActorLocation))
    (else
      (Transformation|SetActorLocation (Math|Vector|Lerp(Vector) (Variables|Default|GetstartPos) (Variables|Default|GetgoalPos) _output_get) false false))))

(fn ConstructionScript)