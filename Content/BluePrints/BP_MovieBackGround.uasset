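; BP_MovieBackGround is an actor that fades a sphere backdrop in and out for movie playback.
; On BeginPlay it creates a dynamic material instance on the Sphere and stores it.
; Each Tick it ramps a clamped alpha up while MovieStart is true and down otherwise, writing it to the material's myAlpha parameter, stopping just short of full value.
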(event EventBeginPlay
  (bind _returnvalue (Rendering|Material|CreateDynamicMaterialInstance (Variables|Default|GetSphere) 0 0 "None" :!class /Script/Engine.PrimitiveComponent))
  (Variables|Default|SetmyMaterial _returnvalue))

(event Collision|EventActorBeginOverlap
  (params (OtherActor :type Actor%20Object%20Reference)))

(event EventTick
  (params (DeltaSeconds :type Float%20%28single-precision%29))
  (bind _returnvalue (* DeltaSeconds 1.0))
  (bind _mymaterial (Variables|Default|GetmyMaterial))
  (if (Variables|Default|GetmovieStart)
    (bind _output_get (Variables|Default|SetcurrentAlpha (Math|Float|Clamp(Float) (+ (Variables|Default|GetcurrentAlpha) _returnvalue) 0.0 0.9)))
    (Rendering|Material|SetScalarParameterValue _mymaterial "myAlpha" _output_get :!class /Script/Engine.MaterialInstanceDynamic)
    (else
      (bind _output_get_2 (Variables|Default|SetcurrentAlpha (Math|Float|Clamp(Float) (- (Variables|Default|GetcurrentAlpha) _returnvalue) 0.0 0.9)))
      (Rendering|Material|SetScalarParameterValue _mymaterial "myAlpha" _output_get_2 :!class /Script/Engine.MaterialInstanceDynamic))))

(fn ConstructionScript)