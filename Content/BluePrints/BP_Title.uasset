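; BP_Title is an actor that animates the title and logo widgets, likely for a title screen.
; On BeginPlay it gets the WBP_Title and WBP_Logo instances from its two widget components and starts a separate timeline for each.
; Each timeline drives the alpha of a color written to its widget's MyColor, and the logo timeline also sets MyAlpha.
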(event EventBeginPlay
  (Utilities|FlowControl|Sequence
    (:then_0
      (bind _aswbp_title (Utilities|Casting|CastToWBP_Title (UserInterface|GetWidget (Variables|Default|GetWidget))))
      (Variables|Default|SetAs%20WBP%20Title _aswbp_title)
      (bind _newtrack_0 (Timeline|Timeline_0 Play)
        (:Update
          (Variables|/Game/BluePrints/WBP_Title.WBP_Title_C|SetmyColor (Variables|Default|GetAs%20WBP%20Title) (Utilities|Struct|MakeSlateColor (Utilities|Struct|MakeLinearColor 0.0 0.0 0.0 _newtrack_0))))))
    (:then_1
      (bind _aswbp_logo (Utilities|Casting|CastToWBP_Logo (UserInterface|GetWidget (Variables|Default|GetWidget2))))
      (bind _newtrack_0_2 (Timeline|Timeline_1 Play)
        (:Update
          (Variables|/Game/BluePrints/WBP_Logo.WBP_Logo_C|SetmyColor _aswbp_logo (Utilities|Struct|MakeSlateColor (Utilities|Struct|MakeLinearColor 0.0 0.0 0.0 _newtrack_0_2)))
          (Variables|/Game/BluePrints/WBP_Logo.WBP_Logo_C|SetmyAlpha _aswbp_logo _newtrack_0_2))))))

(event Collision|EventActorBeginOverlap
  (params (OtherActor :type Actor%20Object%20Reference)))

(fn ConstructionScript)