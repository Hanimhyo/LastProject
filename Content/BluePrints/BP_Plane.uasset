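; BP_Plane is a textured panel actor in a VR scene that fades in, follows a target actor, and can be selected for video playback.
; Tick runs a state machine that lerps toward TargetActor, with Move handing off to Boids, Wait or Select on arrival.
; Select enlarges the plane, then triggers the player's OnPlayVideo and holds it at the target; Cancel shrinks it back.
; BeginPlay creates the dynamic material and ramps travel speed over timed delays.
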(event Custom|GoSelect
  (Variables|Default|Setm_State "NewEnumerator2")
  (Variables|Default|SetcurrentAlpha 0.0)
  (Variables|Default|SetstartPoint (Transformation|GetActorLocation))
  (Variables|Default|Setyeild_State "NewEnumerator4")
  (Variables|Default|SetcurrentSelectTime 0.0))

(event Custom|GoBoids
  (Variables|Default|Setm_State "NewEnumerator2")
  (Variables|Default|SetcurrentAlpha 0.0)
  (Variables|Default|SetstartPoint (Transformation|GetActorLocation))
  (Variables|Default|Setyeild_State "NewEnumerator0"))

(event Custom|GoWait
  (Variables|Default|Setm_State "NewEnumerator2")
  (Variables|Default|SetcurrentAlpha 0.0)
  (Variables|Default|SetstartPoint (Transformation|GetActorLocation))
  (Variables|Default|Setyeild_State "NewEnumerator1")
  (Variables|Default|SetcurrentRandVectorTime 0.0))

(event Custom|GoCancel
  (Variables|Default|Setm_State "NewEnumerator5")
  (Variables|Default|SetcurrentAlpha 0.0)
  (Variables|Default|Setyeild_State "NewEnumerator1"))

(event Custom|SetTexture
  (params (texture :type Texture%202D%20Object%20Reference))
  (Rendering|Material|SetTextureParameterValue (Variables|Default|GetmyMaterial) "MainTexture" texture))

(event Custom|GoStartWait
  (params (firstWaitTime :type Float%20%28single-precision%29) (alphaTime :type Float%20%28single-precision%29))
  (Variables|Default|SetFirstWaitTime firstWaitTime)
  (Variables|Default|SetWaitTime alphaTime))

(event EventBeginPlay
  (Variables|Default|SetstartScale (Variables|/Script/Engine.SceneComponent|GetRelativeScale3D (Variables|Default|GetPlane)))
  (bind _asbp_vrplayer (Utilities|Casting|CastToBP_VRPlayer (Game|Player|GetPlayerPawn 0)))
  (Variables|Default|Setplayer _asbp_vrplayer)
  (bind _returnvalue (Rendering|Material|CreateDynamicMaterialInstance (Variables|Default|GetPlane) 0 0 "None" :!class /Script/Engine.PrimitiveComponent))
  (bind _output_get (Variables|Default|SetmyMaterial _returnvalue))
  (Rendering|Material|SetScalarParameterValue _output_get "MyAlpha" 0.0 :!class /Script/Engine.MaterialInstanceDynamic)
  (Utilities|FlowControl|Delay 18.0)
  (Variables|Default|SetlerpMoveSpeed 0.015)
  (Utilities|FlowControl|Delay 3.0)
  (Variables|Default|SetlerpMoveSpeed 0.03)
  (Utilities|FlowControl|Delay 4.0)
  (Variables|Default|SetlerpMoveSpeed 0.05))

(event Collision|EventActorBeginOverlap
  (params (OtherActor :type Actor%20Object%20Reference)))

(event EventTick
  (params (DeltaSeconds :type Float%20%28single-precision%29))
  (switch Utilities|FlowControl|Switch|SwitchonPlaneEnum (Variables|Default|Getm_State)
    (:NewEnumerator6
      (CallFunction|StartWaitEvent))
    (:NewEnumerator0
      (CallFunction|BoidMove))
    (:NewEnumerator1
      (CallFunction|WaitMove))
    (:NewEnumerator2
      (CallFunction|PlaneMoveLerp))
    (:NewEnumerator3
      (CallFunction|PlayMove))
    (:NewEnumerator4
      (CallFunction|SelectPlayTime))
    (:NewEnumerator5
      (CallFunction|CancelScale))))

(fn ConstructionScript)

(fn PlayerLookRotate
  (Transformation|SetActorRotation (Math|Conversions|RotationFromXVector (Math|Vector|Normalize (- (Transformation|GetActorLocation (Variables|Default|Getplayer)) (Transformation|GetActorLocation))))))

(fn PlaneMoveLerp
  (bind _returnvalue (Transformation|GetActorLocation))
  (bind _targetactor (Variables|Default|GettargetActor))
  (bind _returnvalue_2 (Transformation|GetActorLocation _targetactor))
  (Transformation|SetActorLocationAndRotation (Math|Vector|Lerp(Vector) _returnvalue _returnvalue_2 (Variables|Default|GetlerpMoveSpeed)) (Math|Conversions|RotationFromXVector (Math|Vector|Lerp(Vector) (Transformation|GetActorForwardVector) (Transformation|GetActorForwardVector (Variables|Default|GettargetActor)) 0.05)) false true)
  (if (< (Math|Vector|Distance(Vector) _returnvalue _returnvalue_2) 1e+02)
    (bind _output_get (Variables|Default|Setm_State (Variables|Default|Getyeild_State)))
    (if (Utilities|Enum|Equal(Enum) _output_get "NewEnumerator1")
      (Variables|Default|SetnowPos (Transformation|GetActorLocation))
      (Variables|Default|SetranVector (- (Transformation|GetActorLocation (Variables|Default|GettargetActor)) (Transformation|GetActorLocation))))))

(fn PlaneMove
  (if (< (Variables|Default|GetcurrentAlpha) 1.0)
    (Variables|Default|SetcurrentAlpha (Math|Float|Clamp(Float) (+ (Variables|Default|GetcurrentAlpha) (* (Utilities|Time|GetWorldDeltaSeconds) 1.0))))
    (Transformation|SetActorLocation (Math|Vector|Lerp(Vector) (Variables|Default|GetstartPoint) (Variables|Default|GetgoalPoint) (Variables|Default|GetcurrentAlpha)) false false)
    (Transformation|SetActorRotation (Math|Rotator|Lerp(Rotator) (Transformation|GetActorRotation) (Transformation|GetActorRotation (Variables|Default|GettargetActor)) 0.015))
    (else
      (Transformation|SetActorLocation (Variables|Default|GetgoalPoint) false false)
      (bind _output_get (Variables|Default|Setm_State (Variables|Default|Getyeild_State)))
      (if (Utilities|Enum|Equal(Enum) _output_get "NewEnumerator4")
        _))))

(fn SelectPlayTime
  (bind _plane (Variables|Default|GetPlane))
  (bind _targetactor (Variables|Default|GettargetActor))
  (Utilities|FlowControl|Sequence
    (:then_0
      (Transformation|SetActorLocationAndRotation (Math|Vector|Lerp(Vector) (Transformation|GetActorLocation) (Transformation|GetActorLocation (Variables|Default|GettargetActor)) 0.05) (Math|Rotator|MakeRotfromXZ (Math|Vector|Lerp(Vector) (Transformation|GetActorForwardVector) (Transformation|GetActorForwardVector (Variables|Default|GettargetActor)) 0.05) (Math|Vector|Lerp(Vector) (Transformation|GetActorUpVector) (Transformation|GetActorUpVector (Variables|Default|GettargetActor)) 0.05)))
      (Transformation|SetRelativeScale3D _plane (Math|Vector|Lerp(Vector) (Variables|/Script/Engine.SceneComponent|GetRelativeScale3D _plane) (Variables|Default|GetplayScale) 0.02)))
    (:then_1
      (bind _output_get (Variables|Default|SetcurrentSelectTime (+ (Utilities|Time|GetWorldDeltaSeconds) (Variables|Default|GetcurrentSelectTime))))
      (if (> _output_get 1.5)
        (Default|OnPlayVideo (Variables|Default|Getplayer) self)
        (Variables|Default|Setm_State "NewEnumerator3")
        (Variables|Default|SetcurrentSelectTime 0.0)
        (Transformation|SetActorLocationAndRotation (+ (Transformation|GetActorLocation _targetactor) (* (Transformation|GetActorForwardVector _targetactor) -2.0)) (Transformation|GetActorRotation _targetactor))
        (Transformation|SetRelativeScale3D (Variables|Default|GetPlane) (- (Variables|Default|GetplayScale) 0.01))))))

(fn WaitMove
  (Transformation|SetActorLocationAndRotation (Math|Vector|Lerp(Vector) (Transformation|GetActorLocation) (Transformation|GetActorLocation (Variables|Default|GettargetActor)) 0.05) (Math|Conversions|RotationFromXVector (Math|Vector|Lerp(Vector) (Transformation|GetActorForwardVector) (Transformation|GetActorForwardVector (Variables|Default|GettargetActor)) 0.05)) false true))

(fn BoidMove
  (Transformation|SetActorLocationAndRotation (Math|Vector|Lerp(Vector) (Transformation|GetActorLocation) (Transformation|GetActorLocation (Variables|Default|GettargetActor)) 0.05) (Math|Conversions|RotationFromXVector (Math|Vector|Lerp(Vector) (Transformation|GetActorForwardVector) (Transformation|GetActorForwardVector (Variables|Default|GettargetActor)) 0.01)) false true))

(fn CancelScale
  (if (< (Variables|Default|GetcurrentAlpha) 1.0)
    (bind _output_get (Variables|Default|SetcurrentAlpha (Math|Float|Clamp(Float) (+ (Variables|Default|GetcurrentAlpha) (* (Utilities|Time|GetWorldDeltaSeconds) 2.0)))))
    (Transformation|SetRelativeScale3D (Variables|Default|GetPlane) (Math|Vector|Lerp(Vector) (Variables|Default|GetplayScale) (Variables|Default|GetstartScale) _output_get))
    (else
      (Transformation|SetRelativeScale3D (Variables|Default|GetPlane) (Variables|Default|GetstartScale))
      (Variables|Default|Setm_State (Variables|Default|Getyeild_State))
      (Variables|Default|SetcurrentAlpha 0.0))))

(fn StartWaitEvent
  (bind _waittime (Variables|Default|GetWaitTime))
  (bind _output_get (Variables|Default|SetcurrentFirstTime (+ (Variables|Default|GetcurrentFirstTime) (Utilities|Time|GetWorldDeltaSeconds))))
  (if (> _output_get (Variables|Default|GetFirstWaitTime))
    (bind _output_get_2 (Variables|Default|SetcurrentWaitTime (+ (Variables|Default|GetcurrentWaitTime) (Utilities|Time|GetWorldDeltaSeconds))))
    (if (> _output_get_2 (Variables|Default|GetWaitTime))
      (Rendering|Material|SetScalarParameterValue (Variables|Default|GetmyMaterial) "MyAlpha" 1.0 :!class /Script/Engine.MaterialInstanceDynamic)
      (Variables|Default|SetfirstBoids true)
      (Variables|Default|SetlerpMoveSpeed 0.01)
      (CallFunction|GoBoids)
      (else
        (Rendering|Material|SetScalarParameterValue (Variables|Default|GetmyMaterial) "MyAlpha" (/ (Math|Float|Clamp(Float) (* (Variables|Default|GetcurrentWaitTime) 1.2) 0.0 _waittime) _waittime) :!class /Script/Engine.MaterialInstanceDynamic)))))

(fn PlayMove
  (bind _targetactor (Variables|Default|GettargetActor))
  (Transformation|SetActorLocationAndRotation (+ (Transformation|GetActorLocation _targetactor) (* (Transformation|GetActorForwardVector _targetactor) -2.0)) (Transformation|GetActorRotation _targetactor)))