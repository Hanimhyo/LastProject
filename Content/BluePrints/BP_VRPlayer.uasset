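; VR player that lets the user pick BP_Plane actors and watch their videos on a shared BP_MoviePlane.
; Grip axes drive both hand anim blueprints, while the right trigger line-traces from the hand to select or cancel a plane and clicks widgets when no video plays.
; OnPlayVideo maps the plane's index in BP_PointMaker to a video; cancelling stops it.
; With an HMD enabled, BeginPlay sets floor tracking and finds the scene actors.
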(event Custom|OnPlayVideo
  (params (playPlane :type BP%20Plane%20Object%20Reference))
  (bind _mybp_pointmaker (Variables|Default|GetmyBP_PointMaker))
  (bind _planeactorarray (Variables|/Game/BluePrints/BP_PointMaker.BP_PointMaker_C|GetplaneActorArray _mybp_pointmaker))
  (bind _returnvalue (Utilities|Array|FindItem _planeactorarray playPlane))
  (if (not (== _returnvalue -1))
    (Default|PlayVideo (Variables|Default|GetmyBP_MoviePlane) _returnvalue)
    (Variables|Default|SetisVideoPlay true)))

(event EventBeginPlay
  (if (Class|HeadMountedDisplayFunctionLibrary|IsHeadMountedDisplayEnabled)
    (Class|HeadMountedDisplayFunctionLibrary|SetTrackingOrigin "Floor")
    (CallFunction|StartSetting)))

(event Collision|EventActorBeginOverlap
  (params (OtherActor :type Actor%20Object%20Reference)))

(event EventTick
  (params (DeltaSeconds :type Float%20%28single-precision%29)))

(event Input|ActionEvents|InputActionTriggerRight
  (params (Key :type Key%20Structure :default "None"))
  (bind _widgetinteraction (Variables|Default|GetWidgetInteraction))
  (:Pressed
    (CallFunction|SelectPlane)
    (if (not (Variables|Default|GetisVideoPlay))
      (Class|WidgetInteractionComponent|PressPointerKey _widgetinteraction "LeftMouseButton")))
  (:Released
    (if (not (Variables|Default|GetisVideoPlay))
      (Class|WidgetInteractionComponent|ReleasePointerKey _widgetinteraction "LeftMouseButton"))))

(event Input|AxisEvents|InputAxisGrabAxisLeft
  (params (AxisValue :type Float%20%28single-precision%29))
  (bind _asabp_hand_anim (Utilities|Casting|CastToABP_HandAnim (Components|SkeletalMesh|GetAnimInstance (Variables|Default|GetLeftHandSkeletalMesh))))
  (Variables|/Game/BluePrints/ABP_HandAnim.ABP_HandAnim_C|SetGripValue _asabp_hand_anim AxisValue))

(event Input|AxisEvents|InputAxisGrabAxisRight
  (params (AxisValue :type Float%20%28single-precision%29))
  (bind _asabp_hand_anim (Utilities|Casting|CastToABP_HandAnim (Components|SkeletalMesh|GetAnimInstance (Variables|Default|GetRightHandSkeletalMesh))))
  (Variables|/Game/BluePrints/ABP_HandAnim.ABP_HandAnim_C|SetGripValue _asabp_hand_anim AxisValue))

(fn ConstructionScript)

(fn SelectPlane
  (bind _righthandskeletalmesh (Variables|Default|GetRightHandSkeletalMesh))
  (bind _returnvalue (Transformation|GetWorldLocation _righthandskeletalmesh))
  (bind _outhit (Collision|LineTraceByChannel _returnvalue (+ _returnvalue (* (Math|Vector|GetForwardVector _righthandskeletalmesh) 2e+03)) "TraceTypeQuery1" false 0 "None"))
  (bind _asbp_plane (Utilities|Casting|CastToBP_Plane (.HitActor (Collision|BreakHitResult _outhit))))
  (if (Utilities|Enum|Equal(Enum) (Variables|/Game/BluePrints/BP_Plane.BP_Plane_C|Getm_State _asbp_plane) "NewEnumerator1")
    (if (not (Utilities|IsValid (Variables|Default|GetmyselectPlane)))
      (Default|GoSelect _asbp_plane)
      (Variables|/Game/BluePrints/BP_Plane.BP_Plane_C|SetgoalPoint _asbp_plane (+ (Transformation|GetActorLocation) (* (Transformation|GetActorForwardVector) 2e+02)))
      (Variables|Default|SetmyselectPlane _asbp_plane)
      (Variables|Default|SetselectWaitPosActor (Variables|/Game/BluePrints/BP_Plane.BP_Plane_C|GettargetActor _asbp_plane))
      (Variables|/Game/BluePrints/BP_Plane.BP_Plane_C|SettargetActor _asbp_plane (Variables|Default|GetmyBP_MoviePlane)))
    (elif (Utilities|Enum|Equal(Enum) (Variables|/Game/BluePrints/BP_Plane.BP_Plane_C|Getm_State _asbp_plane) "NewEnumerator3")
      (Default|GoCancel (Variables|Default|GetmyselectPlane))
      (Variables|/Game/BluePrints/BP_Plane.BP_Plane_C|SettargetActor (Variables|Default|GetmyselectPlane) (Variables|Default|GetselectWaitPosActor))
      (Variables|Default|SetmyselectPlane 0)
      (Default|StopVideo (Variables|Default|GetmyBP_MoviePlane))
      (Variables|Default|SetisVideoPlay false))))

(fn StartSetting
  (Utilities|FlowControl|Sequence
    (:then_0
      (bind _outactors (Actor|GetAllActorsOfClass "/Game/BluePrints/BP_MoviePlane.BP_MoviePlane_C"))
      (Variables|Default|SetmyBP_MoviePlane (Utilities|Array|Get(acopy) _outactors)))
    (:then_1
      (bind _outactors_2 (Actor|GetAllActorsOfClass "/Game/BluePrints/BP_PointMaker.BP_PointMaker_C"))
      (Variables|Default|SetmyBP_PointMaker (Utilities|Array|Get(acopy) _outactors_2)))
    (:then_2
      (bind _outactors_3 (Actor|GetAllActorsOfClass "/Game/BluePrints/BP_ArrayMaster.BP_ArrayMaster_C"))
      (Variables|Default|SetmyBp_ArrayMaster (Utilities|Array|Get(acopy) _outactors_3)))))