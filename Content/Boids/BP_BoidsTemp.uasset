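; Boids actor for VR that drives a Niagara flock and pulls it toward the actor while the player holds the left trigger.
; Tick updates the attractor position and lerped strength and toggles the pointer effect.
; Niagara exports particle data back to the actor, which stores positions and velocities in arrays, using particle Size as the index.
; A release event plays a timeline-scaled sphere effect; the RandomPos wander function is never called.
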(event Custom|RelaeseEvent
  (bind _relaesesphere (Variables|Default|GetRelaeseSphere))
  (Rendering|SetVisibility _relaesesphere true false)
  (bind _newtrack_0 (Timeline|Timeline_0 PlayFromStart)
    (:Update
      (Transformation|SetRelativeScale3D _relaesesphere _newtrack_0))
    (:Finished
      (Rendering|SetVisibility _relaesesphere false false))))

(event EventBeginPlay
  (bind _asbp_vrplayer (Utilities|Casting|CastToBP_VRPlayer (Game|Player|GetPlayerPawn 0)))
  (Variables|Default|Setplayer _asbp_vrplayer)
  (Class|NiagaraComponent|SetVariableObject (Variables|Default|GetBoidsNiagara) "PositionObj" self)
  (Variables|Default|SetstartPos (Transformation|GetActorLocation))
  (for _index (range 0 500)
    (Utilities|Array|Add :TargetArray (Variables|Default|GetparticlesPosArray))
    (Utilities|Array|Add :TargetArray (Variables|Default|GetparticleVelArray))))

(event Collision|EventActorBeginOverlap
  (params (OtherActor :type Actor%20Object%20Reference)))

(event EventTick
  (params (DeltaSeconds :type Float%20%28single-precision%29))
  (CallFunction|RandomMove))

(event EventParticleData
  (params (Data :type Array%20of%20Basic%20Particle%20Data%20Structures) (NiagaraSystem :type Niagara%20System%20Object%20Reference))
  (for _array_element Data
    (Utilities|Array|SetArrayElem (Variables|Default|GetparticlesPosArray) (Math|Conversions|ToInteger(Byte) (Class|KismetMathLibrary|Round64 (.Size (Utilities|Struct|BreakBasicParticleData _array_element)))) (.Position (Utilities|Struct|BreakBasicParticleData _array_element)) true)
    (Utilities|Array|SetArrayElem (Variables|Default|GetparticleVelArray) (Math|Conversions|ToInteger(Byte) (Class|KismetMathLibrary|Round64 (.Size (Utilities|Struct|BreakBasicParticleData _array_element)))) (.Velocity (Utilities|Struct|BreakBasicParticleData _array_element)) true)))

(fn ConstructionScript)

(fn RandomPos
  (bind _output_get (Variables|Default|SetcurrentTime (+ (Variables|Default|GetcurrentTime) (* (Utilities|Time|GetWorldDeltaSeconds) 0.2))))
  (if true
    (Variables|Default|SetrandomVector (* (Math|Random|RandomUnitVector) 2e+02))
    (Variables|Default|SetcurrentTime 0.0)
    (else
      (Transformation|SetActorLocation (Math|Vector|Lerp(Vector) (Variables|Default|GetstartPos) (+ (Variables|Default|GetstartPos) (Variables|Default|GetrandomVector)) (Variables|Default|GetcurrentTime)) false false))))

(fn RandomMove
  (bind _boidsniagara (Variables|Default|GetBoidsNiagara))
  (bind _nipointer (Variables|Default|GetNIPointer))
  (if (Variables|/Game/BluePrints/BP_VRPlayer.BP_VRPlayer_C|GetleftTrigger (Variables|Default|Getplayer))
    (Variables|Default|SetgoalStrenght 2e+03)
    (Components|Activation|SetActive _nipointer true false)
    (else
      (Variables|Default|SetgoalStrenght 0.0)
      (Components|Activation|SetActive _nipointer false false)))
  (Niagara|SetNiagaraVariable(Float) _boidsniagara "Attraction Strength" (Math|Float|Lerp (Variables|Default|GetcurrentStrenght) (Variables|Default|GetgoalStrenght) 0.1))
  (Niagara|SetNiagaraVariable(Vector3) _boidsniagara "Attractor Position" (Transformation|GetActorLocation)))